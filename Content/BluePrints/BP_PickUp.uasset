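; BP_PickUp is a pickup actor that spins, bobs and shows a name label when the first-person character is near; it has no collection logic.
; Tick applies yaw rotation scaled by delta time and a sine-based vertical offset added each frame, making the bob frame-rate dependent.
; Overlap begin speeds up the spin and reveals the text; overlap end restores both.
; The construction script applies the selected mesh and name.
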(event EventTick
  (params (DeltaSeconds :type Float%20%28single-precision%29))
  ;[1 1 1] Rotation Pickup
  (Transformation|AddLocalRotation (Variables|Default|GetPickupMesh) (Math|Rotator|MakeRotator 0.0 0.0 (* DeltaSeconds (Variables|Config|GetRotation_Speed))) false false)
  ;[1 1 1] Floating Pickup
  (Transformation|AddRelativeLocation (Variables|Default|GetPickupMesh) (Math|Vector|MakeVector 0.0 0.0 (* (Math|Trig|Sin(Radians) (* (Variables|Default|GetZfrequency) (Utilities|Time|GetGameTimeinSeconds))) (Variables|Default|GetZscale))) false false))

(event Collision|EventActorBeginOverlap
  (params (OtherActor :type Actor%20Object%20Reference))
  ;[1 1 1] Rotacion y texto visible cuando nos acercamos
  (Utilities|Casting|CastToFirstPersonCharacter OtherActor)
  (bind _output_get (Variables|Default|Settmp_RotationSpeed (Variables|Config|GetRotation_Speed)))
  (Variables|Config|SetRotation_Speed (* _output_get 1e+01))
  (Rendering|SetVisibility (Variables|Default|GetTextRender) true false))

(event Collision|EventActorEndOverlap
  (params (OtherActor :type Actor%20Object%20Reference))
  ;[1 1 1] Rotacion y texto visible cuando nos alejamos
  (Utilities|Casting|CastToFirstPersonCharacter OtherActor)
  (Variables|Config|SetRotation_Speed (Variables|Default|Gettmp_RotationSpeed))
  (Rendering|SetVisibility (Variables|Default|GetTextRender) false false))

(fn ConstructionScript
  (Components|StaticMesh|SetStaticMesh (Variables|Default|GetPickupMesh) (Variables|Config|GetSelectMesh))
  (Rendering|Components|TextRender|SetText (Variables|Default|GetTextRender) (Variables|Config|GetName)))